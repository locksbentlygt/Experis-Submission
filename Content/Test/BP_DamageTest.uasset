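; BP_DamageTest is a functional test that checks whether the player character dies while moving forward.
; On start it finds the ExperisCharacter in the level, then each tick feeds it movement input built from the X component of its forward vector.
; The test succeeds once the character's IsDead flag is set; it has no explicit failure branch.
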(event `self.ReceiveStartTest`
  (bind _returnvalue (`GameplayStatics.GetActorOfClass` "/Script/MyProject.ExperisCharacter"))
  (set `self.Character` _returnvalue))

(event `self.ReceiveTick`
  (params (DeltaSeconds :type "Float (single-precision)"))
  (bind _character (`self.Character`))
  (`Pawn.AddMovementInput` _character (`KismetMathLibrary.MakeVector` (.x (`self.GetActorForwardVector` _character))) 5.0 false)
  (if (`ExperisCharacter.IsDead` (`self.Character`))
    (`self.FinishTest` "Succeeded")))

(fn `UserConstructionScript`)